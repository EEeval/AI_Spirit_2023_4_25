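; BP_Computer is an interactive computer with a password-entry screen and a drag-to-rotate spring arm view.
; On BeginPlay it caches the WBP_ComputerScreen from its widget component and adds inventory and PlayerAMain widgets to the viewport.
; Clickable arrow, Enter and IO boxes forward index, number, password and screen-open calls to that screen widget.
; While left mouse is held and EnableRotate is set, horizontal mouse movement yaws the spring arm.
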(event OnClicked(Box_Arror_Up)
  (params (TouchedComponent :type Primitive%20Component%20Object%20Reference) (ButtonPressed :type Key%20Structure :default "None"))
  ;[1 1 1] Control
  (Default|AddNumber (Variables|Default|GetAs%20WBP%20Computer%20Screen)))

(event OnClicked(Box_Arror_Right)
  (params (TouchedComponent :type Primitive%20Component%20Object%20Reference) (ButtonPressed :type Key%20Structure :default "None"))
  ;[1 1 1] Control
  (Default|AddIndex (Variables|Default|GetAs%20WBP%20Computer%20Screen)))

(event OnClicked(Box_Arror_Left)
  (params (TouchedComponent :type Primitive%20Component%20Object%20Reference) (ButtonPressed :type Key%20Structure :default "None"))
  ;[1 1 1] Control
  (Default|SubIndex (Variables|Default|GetAs%20WBP%20Computer%20Screen)))

(event OnClicked(Box_Arror_Down)
  (params (TouchedComponent :type Primitive%20Component%20Object%20Reference) (ButtonPressed :type Key%20Structure :default "None"))
  ;[1 1 1] Control
  (Default|SubNumber (Variables|Default|GetAs%20WBP%20Computer%20Screen)))

(event OnClicked(Box_Arror_Enter)
  (params (TouchedComponent :type Primitive%20Component%20Object%20Reference) (ButtonPressed :type Key%20Structure :default "None"))
  ;[1 1 1] Control
  (Default|EnterPassword (Variables|Default|GetAs%20WBP%20Computer%20Screen)))

(event OnClicked(Box_Arror_IO)
  (params (TouchedComponent :type Primitive%20Component%20Object%20Reference) (ButtonPressed :type Key%20Structure :default "None"))
  ;[1 1 1] Control
  (Default|OpenCompuerScreen (Variables|Default|GetAs%20WBP%20Computer%20Screen)))

(event EventBeginPlay
  (Utilities|FlowControl|Sequence
    (:then_0
      (bind _aswbp_computer_screen (Utilities|Casting|CastToWBP_ComputerScreen (UserInterface|GetWidget (Variables|Default|GetWidget))))
      (Variables|Default|SetAs%20WBP%20Computer%20Screen _aswbp_computer_screen)
      (bind _returnvalue (UserInterface|CreateWidget "/Game/UI/WBP_Inventory.WBP_Inventory_C" 0 (Variables|Default|GetBPC_InventoryComp)))
      (UserInterface|Viewport|AddtoViewport _returnvalue 0))
    (:then_1
      (bind _returnvalue_2 (UserInterface|CreateWidget "/Game/UI/WBP_PlayerAMain.WBP_PlayerAMain_C" 0 self))
      (UserInterface|Viewport|AddtoViewport _returnvalue_2 99))))

(event EventTick
  (params (DeltaSeconds :type Float%20%28single-precision%29))
  (Utilities|FlowControl|Sequence
    (:then_0
      (if (Variables|Default|GetbEnableDrug)
        (bind _returnvalue (Class|WidgetLayoutLibrary|GetMousePositiononViewport))
        (if (Variables|Default|GetbEnableRotate)
          (Transformation|AddRelativeRotation (Variables|Default|GetSpringArm) (Math|Rotator|MakeRotator 0.0 0.0 (* (.X (Math|Vector2D|BreakVector2D (- _returnvalue (Variables|Default|GetLastMousePosition)))) 0.5)) false false))
        (Variables|Default|SetLastMousePosition _returnvalue)))))

(event Input|MouseEvents|LeftMouseButton
  (params (Key :type Key%20Structure :default "None"))
  (:Pressed
    (Variables|Default|SetbEnableDrug true)
    (bind _returnvalue (Class|WidgetLayoutLibrary|GetMousePositiononViewport))
    (Variables|Default|SetLastMousePosition _returnvalue))
  (:Released
    (Variables|Default|SetbEnableDrug false)))

(fn ConstructionScript)