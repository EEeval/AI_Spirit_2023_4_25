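; BP_StaticCameraPosition is a clickable viewpoint actor that becomes the player's view target when its Box is clicked.
; The click also turns off EnableRotate on BP_Computer and disables the Box's collision.
; On BeginPlay it finds BP_Computer and binds to its ViewCameraIn event, which restores the Box's query and physics collision so it can be clicked again.
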(event OnClicked(Box)
  (params (TouchedComponent :type Primitive%20Component%20Object%20Reference) (ButtonPressed :type Key%20Structure :default "None"))
  (Variables|/Game/Blueprints/BP_Computer.BP_Computer_C|SetbEnableRotate (Variables|Default|GetBP_Computer) false)
  (Collision|SetCollisionEnabled (Variables|Default|GetBox) "NoCollision")
  (Game|Player|SetViewTargetwithBlend (Game|GetPlayerController 0) self 0.0 "VTBlend_Linear" 0.0 false))

(event Custom|EnableCollision
  (Collision|SetCollisionEnabled (Variables|Default|GetBox) "QueryAndPhysics"))

(event EventBeginPlay
  (bind _returnvalue (Actor|GetActorOfClass "/Game/Blueprints/BP_Computer.BP_Computer_C"))
  (bind _output_get (Variables|Default|SetBP_Computer _returnvalue))
  (EventDispatchers|BindEventtoViewCamerain _output_get (delegate Custom|EnableCollision)))

(event Collision|EventActorBeginOverlap
  (params (OtherActor :type Actor%20Object%20Reference)))

(event EventTick
  (params (DeltaSeconds :type Float%20%28single-precision%29)))

(fn ConstructionScript)