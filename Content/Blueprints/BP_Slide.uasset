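; BP_Slide is an actor with three mouse-dragged slider buttons (top, middle, bottom) that snap to seven positions along local X.
; Pressing a button stores its index, and releasing it or the static mesh clears it.
; Seven boxes act as cursor hover zones, passing their slot to SetButtonLocationWithIndex, which moves the selected button and prints the slot.
; BeginPlay places the top button in the last slot.
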(event OnBeginCursorOver(Box)
  (params (TouchedComponent :type Primitive%20Component%20Object%20Reference))
  (CallFunction|SetButtonLocationwithIndex (Variables|Default|GetChoosenButtonIndex)))

(event OnBeginCursorOver(Box6)
  (params (TouchedComponent :type Primitive%20Component%20Object%20Reference))
  (CallFunction|SetButtonLocationwithIndex (Variables|Default|GetChoosenButtonIndex) 6))

(event OnReleased(Button_Mid)
  (params (TouchedComponent :type Primitive%20Component%20Object%20Reference) (ButtonReleased :type Key%20Structure :default "None"))
  (Variables|Default|SetChoosenButtonIndex -1))

(event OnClicked(Button_Bot)
  (params (TouchedComponent :type Primitive%20Component%20Object%20Reference) (ButtonPressed :type Key%20Structure :default "None"))
  (Variables|Default|SetChoosenButtonIndex 0))

(event OnReleased(Button_Bot)
  (params (TouchedComponent :type Primitive%20Component%20Object%20Reference) (ButtonReleased :type Key%20Structure :default "None"))
  (Variables|Default|SetChoosenButtonIndex -1))

(event OnReleased(StaticMesh)
  (params (TouchedComponent :type Primitive%20Component%20Object%20Reference) (ButtonReleased :type Key%20Structure :default "None"))
  (Variables|Default|SetChoosenButtonIndex -1))

(event OnBeginCursorOver(Box1)
  (params (TouchedComponent :type Primitive%20Component%20Object%20Reference))
  (CallFunction|SetButtonLocationwithIndex (Variables|Default|GetChoosenButtonIndex) 1))

(event OnBeginCursorOver(Box2)
  (params (TouchedComponent :type Primitive%20Component%20Object%20Reference))
  (CallFunction|SetButtonLocationwithIndex (Variables|Default|GetChoosenButtonIndex) 2))

(event OnBeginCursorOver(Box3)
  (params (TouchedComponent :type Primitive%20Component%20Object%20Reference))
  (CallFunction|SetButtonLocationwithIndex (Variables|Default|GetChoosenButtonIndex) 3))

(event OnBeginCursorOver(Box4)
  (params (TouchedComponent :type Primitive%20Component%20Object%20Reference))
  (CallFunction|SetButtonLocationwithIndex (Variables|Default|GetChoosenButtonIndex) 4))

(event OnBeginCursorOver(Box5)
  (params (TouchedComponent :type Primitive%20Component%20Object%20Reference))
  (CallFunction|SetButtonLocationwithIndex (Variables|Default|GetChoosenButtonIndex) 5))

(event OnClicked(Button_Top)
  (params (TouchedComponent :type Primitive%20Component%20Object%20Reference) (ButtonPressed :type Key%20Structure :default "None"))
  (Variables|Default|SetChoosenButtonIndex 2))

(event OnReleased(Button_Top)
  (params (TouchedComponent :type Primitive%20Component%20Object%20Reference) (ButtonReleased :type Key%20Structure :default "None"))
  (Variables|Default|SetChoosenButtonIndex -1))

(event OnClicked(Button_Mid)
  (params (TouchedComponent :type Primitive%20Component%20Object%20Reference) (ButtonPressed :type Key%20Structure :default "None"))
  (Variables|Default|SetChoosenButtonIndex 1))

(event EventBeginPlay
  (CallFunction|SetButtonLocationwithIndex 2 6))

(event Collision|EventActorBeginOverlap
  (params (OtherActor :type Actor%20Object%20Reference)))

(event EventTick
  (params (DeltaSeconds :type Float%20%28single-precision%29)))

(fn ConstructionScript)

(fn SetButtonLocationwithIndex
  (params (ButtonIndex :type Integer) (LocationIndex :type Integer))
  (switch int ButtonIndex
    (:0
      (LocalVariables|SetMovingComponent (Variables|Default|GetButton_Bot)))
    (:1
      (LocalVariables|SetMovingComponent (Variables|Default|GetButton_Mid)))
    (:2
      (LocalVariables|SetMovingComponent (Variables|Default|GetButton_Top)))
    (:3
      (return)))
  (Transformation|SetRelativeLocation (LocalVariables|GetMovingComponent) (Math|Vector|MakeVector (Math|Conversions|ToFloat(Integer) (* (- LocationIndex 3) 5)) 0.0 0.0) false false)
  (Development|PrintString (Utilities|String|ToString(Integer) LocationIndex)))