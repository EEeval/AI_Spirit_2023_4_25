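; BP_Inventory is an inventory Blueprint that stores items as structs in a slot array, with custom events to initialize, add and remove.
; CE_InitItems appends a fixed number of empty items, and CE_RemoveItem overwrites the slot at a given index with the empty item.
; CE_AddItem copies the new item's fields into every element with a non-zero Id, without stopping, so zero-Id slots are never filled.
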(event Custom|CE_AddItem
  (params (NewItem :type S%20Inventory%20Item%20Structure%20%28by%20ref%29))
  (bind (_id _name _icon _mesh) (Utilities|Struct|BreakS_InventoryItem NewItem))
  (for _array_element (Variables|Default|GetInventoryItems)
    (if (!= (.Id (Utilities|Struct|BreakS_InventoryItem _array_element)) 0)
      (Utilities|Struct|SetmembersinS_InventoryItem _array_element _id _name _icon _mesh))))

(event Custom|CE_RemoveItem
  (params (IndexToRemove :type Integer))
  (|SetBy-RefVar (Utilities|Array|Get(acopy) (Variables|Default|GetInventoryItems) IndexToRemove) (Variables|Default|GetEmptyItem)))

(event Custom|CE_InitItems
  (for _index (range 0 10)
    (Utilities|Array|Add (Variables|Default|GetInventoryItems) (Variables|Default|GetEmptyItem))))

(event EventBeginPlay)

(event Collision|EventActorBeginOverlap
  (params (OtherActor :type Actor%20Object%20Reference)))

(event EventTick
  (params (DeltaSeconds :type Float%20%28single-precision%29)))

(fn ConstructionScript)