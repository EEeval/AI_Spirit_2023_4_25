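; Inventory component that stores items in a fixed number of slots, with an Id of 0 marking a free slot.
; CE_InitItems fills InventoryItems with EmptyItem up to InventorySize.
; CE_AddItem copies an item into the first free slot, while CE_RemoveItem targets the first matching Id for clearing.
; Both edit structs in place and then fire their dispatchers, even when no slot matched.
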(event Custom|CE_RemoveItem
  (params (ItemIdToRemove :type Integer))
  (bind _inventoryitems (Variables|Default|GetInventoryItems))
  (bind (_array_element _array_index) (Utilities|Array|ForEachLoopwithBreak _inventoryitems :!label _label)
    (:LoopBody
      (if (== (Utilities|Struct|BreakS_InventoryItem _array_element) ItemIdToRemove)
        (Utilities|Struct|SetmembersinS_InventoryItem (Utilities|Array|Get(acopy) _inventoryitems _array_index) 0 "" 0 0)
        (goto _label Break)))
    (:Completed
      (Default|CallRemoveItemDispatcher))))

(event Custom|CE_InitItems
  (for _index (range 0 (- (Variables|Default|GetInventorySize) 1))
    (Utilities|Array|Add (Variables|Default|GetInventoryItems) (Variables|Default|GetEmptyItem))))

(event Custom|CE_AddItem
  (params (NewItem :type S%20Inventory%20Item%20Structure%20%28by%20ref%29))
  (bind (_id _name _icon _mesh) (Utilities|Struct|BreakS_InventoryItem NewItem))
  (bind _inventoryitems (Variables|Default|GetInventoryItems))
  (bind (_array_element _array_index) (Utilities|Array|ForEachLoopwithBreak _inventoryitems :!label _label)
    (:LoopBody
      (if (== (Utilities|Struct|BreakS_InventoryItem _array_element) 0)
        (Utilities|Struct|SetmembersinS_InventoryItem (Utilities|Array|Get(acopy) _inventoryitems _array_index) _id _name _icon _mesh)
        (goto _label Break)))
    (:Completed
      (Default|CallAddItemDispatcher))))

(event EventBeginPlay)

(event EventTick
  (params (DeltaSeconds :type Float%20%28single-precision%29)))